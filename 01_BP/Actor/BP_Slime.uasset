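; BP_Slime is a slime actor that damages the player through its Body and can be defeated through its KillPoint.
; Body overlap calls OnLoseHP on man_Character_1 and disables KillPoint collision until the overlap ends.
; A player hit on KillPoint changes CurState, disables both components' collision and spawns a Can_Shoot actor once.
; The spawned actor's sphere collision stays off briefly before being re-enabled.
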(event `self.KillPoint.OnComponentHit`
  (params (HitComponent :type "PrimitiveComponent Object Reference") (OtherActor :type "Actor Object Reference") (OtherComp :type "PrimitiveComponent Object Reference") (NormalImpulse :type "Vector Structure") (Hit :type "HitResult Structure (by ref)"))
  (if (not (`self.IsOverlapPlayer?`))
    (cast `/Game/MY/01_BP/Actor/man_Character_1` OtherActor)
    (`|ExecutionSequence`
      (:`then_0`
        (set `self.Cur_State` "NewEnumerator2")
        (`/Engine/EditorBlueprintResources/StandardMacros.DoOnce` false
          (:`Completed`
            (bind _returnvalue (`|SpawnActorFromClass` "/Game/MY/01_BP/Actor/Can_Shoot.Can_Shoot_C" (`self.GetTransform`) "Undefined" "OverrideRootScale" null null))
            (bind _ascan_shoot (cast `/Game/MY/01_BP/Actor/Can_Shoot` _returnvalue))
            (bind _sphere (`/Game/MY/01_BP/Actor/Can_Shoot.Sphere` _ascan_shoot))
            (`PrimitiveComponent.SetCollisionEnabled` _sphere "NoCollision")
            (`KismetSystemLibrary.Delay` 0.5)
            (`PrimitiveComponent.SetCollisionEnabled` _sphere "QueryAndPhysics"))))
      (:`then_1`
        (`PrimitiveComponent.SetCollisionEnabled` (`self.KillPoint`) "NoCollision")
        (`PrimitiveComponent.SetCollisionEnabled` (`self.Body`) "NoCollision")))))

(event `self.Body.OnComponentBeginOverlap`
  (params (OverlappedComponent :type "PrimitiveComponent Object Reference") (OtherActor :type "Actor Object Reference") (OtherComp :type "PrimitiveComponent Object Reference") (OtherBodyIndex :type Integer) (bFromSweep :type Boolean) (SweepResult :type "HitResult Structure (by ref)"))
  (bind _asman_character_1 (cast `/Game/MY/01_BP/Actor/man_Character_1` OtherActor))
  (`|ExecutionSequence`
    (:`then_0`
      (`/Engine/EditorBlueprintResources/StandardMacros.DoOnce` false :!label _label
        (:`Completed`
          (`/Game/MY/01_BP/Actor/man_Character_1.OnLoseHP` _asman_character_1))))
    (:`then_1`
      (goto _label :!via `Reset`))
    (:`then_2`
      (`PrimitiveComponent.SetCollisionEnabled` (`self.KillPoint`) "NoCollision"))))

(event `self.Body.OnComponentEndOverlap`
  (params (OverlappedComponent :type "PrimitiveComponent Object Reference") (OtherActor :type "Actor Object Reference") (OtherComp :type "PrimitiveComponent Object Reference") (OtherBodyIndex :type Integer))
  (`PrimitiveComponent.SetCollisionEnabled` (`self.KillPoint`) "QueryAndPhysics"))

(fn `UserConstructionScript`
  (`parent.UserConstructionScript`))