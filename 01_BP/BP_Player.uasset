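; BP_Player is the player character, with sideways movement, jumping and a running coin total.
; Two axis inputs add movement along world Y, each scaled by its own speed variable, and the Jump action triggers the jump.
; A coin event adds the incoming value to Howmuch, then passes the new total on through a GetCoinEvent call.
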(event `InputAxis|move_left`
  (params (AxisValue :type "Float (single-precision)"))
  (`self.AddMovementInput` (`KismetMathLibrary.MakeVector` 0.0 (`self.Speed`)) AxisValue))

(event `InputAxis|move_right`
  (params (AxisValue :type "Float (single-precision)"))
  (`self.AddMovementInput` (`KismetMathLibrary.MakeVector` 0.0 (`self.Speed1`)) AxisValue))

(event `InputAction|Jump`
  (params (Key :type "Key Structure"))
  (:`Pressed`
    (`self.Jump`)))

(event `GetCoinEvent_0`
  (params (CoinValue :type Integer))
  (bind _output_get (set `self.Howmuch` (+ CoinValue (`self.Howmuch`))))
  (`self.GetCoinEvent` _output_get))

(fn `UserConstructionScript`)